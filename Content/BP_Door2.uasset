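; BP_Door2 is a door actor that shows an exit prompt widget while the player stands near it.
; BeginPlay creates the P_exit widget, and the Box trigger adds it to the viewport or removes it as the player character enters or leaves.
; PickUpKey sets a HasKey flag, which Interact checks, though that branch does nothing yet.
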(event `self.Box.OnComponentBeginOverlap`
  (params (OverlappedComponent :type "PrimitiveComponent Object Reference") (OtherActor :type "Actor Object Reference") (OtherComp :type "PrimitiveComponent Object Reference") (OtherBodyIndex :type Integer) (bFromSweep :type Boolean) (SweepResult :type "HitResult Structure (by ref)"))
  (if (== OtherActor (`GameplayStatics.GetPlayerCharacter` 0))
    (`UserWidget.AddToViewport` (`self.P_exit`) 0)))

(event `self.Box.OnComponentEndOverlap`
  (params (OverlappedComponent :type "PrimitiveComponent Object Reference") (OtherActor :type "Actor Object Reference") (OtherComp :type "PrimitiveComponent Object Reference") (OtherBodyIndex :type Integer))
  (if (== (`GameplayStatics.GetPlayerCharacter` 0) OtherActor)
    (`Widget.RemoveFromParent` (`self.P_exit`))))

(event `self.ReceiveBeginPlay`
  ;[1 1 1] Appelle le texte en variable
  (bind _returnvalue (`|CreateWidget` "/Game/P_exit.P_exit_C"))
  (set `self.P_exit` _returnvalue))

(event `/Game/BPI_interact.Interact`
  (if (`self.Has Key?`)
    _))

(event `/Game/BPI_Door.PickUpKey`
  (set `self.Has Key?` true))

(fn `UserConstructionScript`)