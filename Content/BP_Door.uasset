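; BP_Door is a key-locked door that swings open and closed when interacted with.
; PickUpKey sets HasKey, which lets Interact alternate through a FlipFlop between playing and reversing a timeline that lerps the mesh's yaw over a quarter turn.
; The Rr overlap component shows the P_Interact2 prompt, created at BeginPlay, while the player character is inside, and removes it on exit.
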(event `/Game/BPI_interact.Interact`
  ;[1 1 1] Gère l'ouverture de la porte
  (if (`self.Has Key ? `)
    (`/Engine/EditorBlueprintResources/StandardMacros.FlipFlop`
      (:`A`
        (bind (_direction _door_track) (`Timeline|Door Timeline` :!label _label)
          (:`Update`
            (`SceneComponent.K2_SetRelativeRotation` (`self.StaticMesh`) (`KismetMathLibrary.MakeRotator` 0.0 0.0 (`KismetMathLibrary.Lerp` 0.0 -90.0 _door_track)) false false))))
      (:`B`
        (goto _label :!via `Reverse`)))))

(event `/Game/BPI_Door.PickUpKey`
  ;[1 1 1] Gère l'ouverture de la porte
  (set `self.Has Key ? ` true))

(event `self.rr.OnComponentBeginOverlap`
  (params (OverlappedComponent :type "PrimitiveComponent Object Reference") (OtherActor :type "Actor Object Reference") (OtherComp :type "PrimitiveComponent Object Reference") (OtherBodyIndex :type Integer) (bFromSweep :type Boolean) (SweepResult :type "HitResult Structure (by ref)"))
  ;[1 1 1] Gère l'affichage du texte "intéragir"
  (if (== OtherActor (`GameplayStatics.GetPlayerCharacter` 0))
    (`UserWidget.AddToViewport` (`self.Interact Prompt 2`) 0)))

(event `self.rr.OnComponentEndOverlap`
  (params (OverlappedComponent :type "PrimitiveComponent Object Reference") (OtherActor :type "Actor Object Reference") (OtherComp :type "PrimitiveComponent Object Reference") (OtherBodyIndex :type Integer))
  ;[1 1 1] Gère l'affichage du texte "intéragir"
  (if (== (`GameplayStatics.GetPlayerCharacter` 0) OtherActor)
    (`Widget.RemoveFromParent` (`self.Interact Prompt 2`))))

(event `self.ReceiveBeginPlay`
  ;[1 1 1] Appelle le texte en variable
  (bind _returnvalue (`|CreateWidget` "/Game/P_Interact2.P_Interact2_C"))
  (set `self.Interact Prompt 2` _returnvalue))

(fn `UserConstructionScript`)