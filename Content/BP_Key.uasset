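; BP_Key is a key pickup actor tied to a Door reference.
; On BeginPlay it creates a P_Interact prompt widget, which is shown while the player character overlaps its Box and removed when the overlap ends.
; Its Interact event calls PickUpKeyMessage on the Door, then destroys the key.
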(event `/Game/BPI_interact.Interact`
  ;[1 1 1] Détruit la clef après l'avoir pick
  (message `/Game/BPI_Door.PickUpKey` (`self.Door`))
  (`self.K2_DestroyActor`))

(event `self.ReceiveBeginPlay`
  ;[1 1 1] Appelle la variable du prompte de la clef
  (bind _returnvalue (`|CreateWidget` "/Game/P_Interact.P_Interact_C"))
  (set `self.Interact Prompt` _returnvalue))

(event `self.Box.OnComponentBeginOverlap`
  (params (OverlappedComponent :type "PrimitiveComponent Object Reference") (OtherActor :type "Actor Object Reference") (OtherComp :type "PrimitiveComponent Object Reference") (OtherBodyIndex :type Integer) (bFromSweep :type Boolean) (SweepResult :type "HitResult Structure (by ref)"))
  ;[1 1 1] Gère le texte "clef"
  (if (== OtherActor (`GameplayStatics.GetPlayerCharacter` 0))
    (`UserWidget.AddToViewport` (`self.Interact Prompt`) 0)))

(event `self.Box.OnComponentEndOverlap`
  (params (OverlappedComponent :type "PrimitiveComponent Object Reference") (OtherActor :type "Actor Object Reference") (OtherComp :type "PrimitiveComponent Object Reference") (OtherBodyIndex :type Integer))
  ;[1 1 1] Gère le texte "clef"
  (if (== (`GameplayStatics.GetPlayerCharacter` 0) OtherActor)
    (`Widget.RemoveFromParent` (`self.Interact Prompt`))))

(fn `UserConstructionScript`)