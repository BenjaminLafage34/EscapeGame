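; BP_Jaques is a Blueprint that shows an on-screen interaction prompt while the player is near it.
; It creates a P_interact3 widget on BeginPlay and keeps it for reuse.
; The Box component's overlap events add the widget to the viewport when player character 0 enters and remove it on exit.
; The file holds only prompt display logic, with no input handling.
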(event `self.Box.OnComponentBeginOverlap`
  (params (OverlappedComponent :type "PrimitiveComponent Object Reference") (OtherActor :type "Actor Object Reference") (OtherComp :type "PrimitiveComponent Object Reference") (OtherBodyIndex :type Integer) (bFromSweep :type Boolean) (SweepResult :type "HitResult Structure (by ref)"))
  ;[1 1 1] Gere le texte du caca
  (if (== OtherActor (`GameplayStatics.GetPlayerCharacter` 0))
    (`UserWidget.AddToViewport` (`self.Interact Prompt 3`) 0)))

(event `self.Box.OnComponentEndOverlap`
  (params (OverlappedComponent :type "PrimitiveComponent Object Reference") (OtherActor :type "Actor Object Reference") (OtherComp :type "PrimitiveComponent Object Reference") (OtherBodyIndex :type Integer))
  ;[1 1 1] Gere le texte du caca
  (if (== (`GameplayStatics.GetPlayerCharacter` 0) OtherActor)
    (`Widget.RemoveFromParent` (`self.Interact Prompt 3`))))

(event `self.ReceiveBeginPlay`
  ;[1 1 1] Gere le texte du caca
  (bind _returnvalue (`|CreateWidget` "/Game/P_interact3.P_interact3_C"))
  (set `self.Interact Prompt 3` _returnvalue))

(fn `UserConstructionScript`)